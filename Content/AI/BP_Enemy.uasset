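; Melee enemy character with an overhead or attached health widget, montage-driven sword and big attacks, and ragdoll death.
; Incoming damage lowers a stat in BPCStats, which is given the widget's health bar.
; Begin/EndSwordTrace toggle a looping timer that sphere-traces between two sword points, throttling hits with DoOnce and a delay.
; PointDamageTrace applies one-shot radius damage, and both traces leave debug drawing on.
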(event `self.ReceiveBeginPlay`
  (bind _aswbp_enemy_health (cast `/Game/UI/WBP_EnemyHealth` (`WidgetComponent.GetWidget` (`self.Widget`))))
  (`/Game/Blueprints/BPC_Stats.SetHealthProgressBar` (`self.BPC_Stats`) (`/Game/UI/WBP_EnemyHealth.HealthBar` _aswbp_enemy_health)))

(event `self.ReceiveAnyDamage`
  (params (Damage :type "Float (single-precision)") (DamageType :type "DamageType Object Reference") (InstigatedBy :type "Controller Object Reference") (DamageCauser :type "Actor Object Reference"))
  (`/Game/Blueprints/BPC_Stats.IncreaseValue` (`self.BPC_Stats`) "NewEnumerator0" (* Damage -1.0)))

(event `/Game/Blueprints/BPI_Damage.End Sword Trace`
  ;[0.5 0.5 0.5] Sword Traces
  (if (`KismetSystemLibrary.K2_IsValidTimerHandle` (stale `/Game/Blueprints/BPI_Damage.Begin Sword Trace` _returnvalue))
    (`KismetSystemLibrary.K2_ClearAndInvalidateTimerHandle` (stale `/Game/Blueprints/BPI_Damage.Begin Sword Trace` _returnvalue))))

(event `/Game/Blueprints/BPI_Damage.Begin Sword Trace`
  ;[0.5 0.5 0.5] Sword Traces
  (bind _returnvalue (`KismetSystemLibrary.K2_SetTimerDelegate` (delegate `DamageTrace`) 0.01 true)))

(event `DamageTrace`
  ;[0.5 0.5 0.5] Sword Traces
  (if (not (`self.isDead`))
    (bind (_outhit _returnvalue) (`KismetSystemLibrary.SphereTraceSingleForObjects` :`Start` (`SceneComponent.K2_GetComponentLocation` (`self.Start Sword Trace Pos`)) :`End` (`SceneComponent.K2_GetComponentLocation` (`self.End Sword Trace Pos`)) :`Radius` 20.0 :`ObjectTypes` (`|MakeArray` "ObjectTypeQuery3" :!type "EObjectTypeQuery Enum") :`DrawDebugType` "ForOneFrame"))
    (if _returnvalue
      (`/Engine/EditorBlueprintResources/StandardMacros.DoOnce` false :!label _label
        (:`Completed`
          (`GameplayStatics.ApplyDamage` (`.HitActor` (`GameplayStatics.BreakHitResult` _outhit)) (`self.Sword Damage`))
          (`KismetSystemLibrary.Delay` 0.3)
          (goto _label :!via `Reset`))))))

(event `/Game/Blueprints/BPI_Damage.Die`
  (`CharacterMovementComponent.DisableMovement` (`self.CharacterMovement`))
  (`PrimitiveComponent.SetSimulatePhysics` (`self.Mesh`) true)
  (set `self.isDead` true))

(event `/Game/AI/BPI_Enemy.Point Damage Trace`
  (bind _returnvalue (`SceneComponent.K2_GetComponentLocation` (`self.Point Trace Pos`)))
  (bind (_outhit _returnvalue_2) (`KismetSystemLibrary.SphereTraceSingleForObjects` :`Start` _returnvalue :`End` _returnvalue :`Radius` (`self.pointBigAttackRadius`) :`ObjectTypes` (`|MakeArray` "ObjectTypeQuery3" :!type "EObjectTypeQuery Enum") :`DrawDebugType` "ForDuration" :`DrawTime` 1.0))
  (if _returnvalue_2
    (`GameplayStatics.ApplyDamage` (`.HitActor` (`GameplayStatics.BreakHitResult` _outhit)) 10.0)))

(fn `BigAttack`
  (returns (Duration :type "Float (double-precision)"))
  (`self.PlayAnimMontage` "/Game/Characters/Souls/Combat/BigAttack_Montage.BigAttack_Montage")
  (return 0.0))

(fn `SwordAttack`
  (returns (Duration :type "Float (double-precision)"))
  (bind _returnvalue (`self.PlayAnimMontage` "/Game/Characters/Souls/Combat/SwordAttackCombo_Montage.SwordAttackCombo_Montage"))
  (return _returnvalue))

(fn `UserConstructionScript`)